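; BP_Item_Child is an item Blueprint that shows a pickup prompt when the player character comes within range.
; On BeginPlay it creates a PickUpText widget, registers itself in its ItemInfo struct, passes the item and prompt text to the widget, and caches the BP_GG player.
; Trigger overlaps with BP_GG add or remove the widget and toggle InRange; the pickup itself is not handled here.
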(event `self.ReceiveBeginPlay`
  (bind _iteminfo (`self.ItemInfo`))
  (bind _pick_up_reference (`self.Pick Up Reference`))
  (bind (_item _itemimage _textpickup) (break `/Game/Main/Levels/Level0/Kentik/HUD/StructurInvent` _iteminfo))
  ;[1 1 1] Event Begin Play
  (bind _returnvalue (`|CreateWidget` "/Game/Main/GG/PickUpText.PickUpText_C"))
  (set `self.Pick Up Reference` _returnvalue)
  (setmembers `/Game/Main/Levels/Level0/Kentik/HUD/StructurInvent` :`StructRef` _iteminfo :`Item` self)
  (set `/Game/Main/GG/PickUpText.PickUpActor` _item _pick_up_reference)
  (set `/Game/Main/GG/PickUpText.TextPickUP` _textpickup _pick_up_reference)
  (bind _asbp_gg (cast `/Game/Main/Levels/Level0/Kentik/HUD/BP_GG` (`GameplayStatics.GetPlayerCharacter` 0)))
  (set `self.As BP GG` _asbp_gg))

(event `self.Trigger.OnComponentBeginOverlap`
  (params (OverlappedComponent :type "PrimitiveComponent Object Reference") (OtherActor :type "Actor Object Reference") (OtherComp :type "PrimitiveComponent Object Reference") (OtherBodyIndex :type Integer) (bFromSweep :type Boolean) (SweepResult :type "HitResult Structure (by ref)"))
  ;[1 1 1] Triger Overla[ Script
  (cast `/Game/Main/Levels/Level0/Kentik/HUD/BP_GG` OtherActor)
  (`UserWidget.AddToViewport` (`self.Pick Up Reference`) 0)
  (set `self.InRange?` true))

(event `self.Trigger.OnComponentEndOverlap`
  (params (OverlappedComponent :type "PrimitiveComponent Object Reference") (OtherActor :type "Actor Object Reference") (OtherComp :type "PrimitiveComponent Object Reference") (OtherBodyIndex :type Integer))
  ;[1 1 1] Triger Overla[ Script
  (cast `/Game/Main/Levels/Level0/Kentik/HUD/BP_GG` OtherActor)
  (`Widget.RemoveFromParent` (`self.Pick Up Reference`))
  (set `self.InRange?` false))

(fn `UserConstructionScript`
  (`parent.UserConstructionScript`))