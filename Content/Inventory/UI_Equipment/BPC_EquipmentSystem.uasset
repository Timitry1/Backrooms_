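; BPC_EquipmentSystem is an equipment component that spawns an item's world actor and attaches it to the player's mesh.
; Initialization stores the Player reference.
; SpawnItemAndAttach spawns the class returned by the item object, keeps it as Hand, snaps it to the socket named on the spawned actor, and passes it the item object.
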(fn `Initialization`
  (params (Player :type "/Game/Main/Levels/Level0/Kentik/HUD/BP_GG Object Reference"))
  (set `self.Player` Player))

(fn `SpawnItemAndAttach`
  (params (ItemObject :type "/Game/Inventory/Inventory2/BP_BaseItemObject Object Reference"))
  (bind _returnvalue (`|SpawnActorFromClass` (`/Game/Inventory/Inventory2/BP_BaseItemObject.GetEquipmentClass` ItemObject) (`KismetMathLibrary.MakeTransform` (0.0 0.0 0.0)) "Undefined" "OverrideRootScale" null null))
  (set `self.Hand` _returnvalue)
  (`Actor.K2_AttachToComponent` _returnvalue (`Character.Mesh` (`self.Player`)) (`/Game/Inventory/UI_Equipment/BP_BaseEquipmentItem.SocketAttach` _returnvalue) "SnapToTarget" "SnapToTarget" "SnapToTarget" true)
  (set `/Game/Inventory/UI_Equipment/BP_BaseEquipmentItem.ItemObject` (`local.ItemObject`) _returnvalue))