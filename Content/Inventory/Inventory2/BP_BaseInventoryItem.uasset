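; BP_BaseInventoryItem is the base world actor for an item that can be picked up into a grid-based inventory.
; On BeginPlay, it builds a default BP_BaseItemObject from its own properties and class, unless a valid one is already set.
; Interact tries auto-stacking into the given inventory component, then falls back to adding a new item.
; On success, it adds the weight and destroys the actor through ServerDestroyItem.
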(event `self.ReceiveBeginPlay`
  (if (not (`KismetSystemLibrary.IsValid` (`self.ItemObject`)))
    (bind _itemobject (`self.GetDefoultItemObject`))
    (set `self.ItemObject` _itemobject)))

(event `/Game/Inventory/Inventory2/BP_Interact.Interact`
  (params (InventoryComponent :type "/Game/Inventory/Inventory2/BPC_Inventory Object Reference"))
  (bind _stack_ (`/Game/Inventory/Inventory2/BPC_Inventory.CheckToAutoStack` InventoryComponent (`self.ItemObject`)))
  (if _stack_
    (`/Game/Inventory/Inventory2/BPC_Inventory.AddWeight` InventoryComponent (`self.ItemObject`) :!label _label)
    (`self.ServerDestroyItem`)
    (else
      (bind _added (`/Game/Inventory/Inventory2/BPC_Inventory.TryAddItem` InventoryComponent (`self.ItemObject`)))
      (if _added
        (goto _label)))))

(event `ServerDestroyItem`
  (`self.K2_DestroyActor`))

(fn `GetDefoultItemObject`
  (returns (ItemObject :type "/Game/Inventory/Inventory2/BP_BaseItemObject Object Reference"))
  (bind (_itemsize_x _itemsize_y) (`KismetMathLibrary.BreakVector2D` (`self.ItemSize`)))
  (bind _returnvalue (`|GenericCreateObject` "/Game/Inventory/Inventory2/BP_BaseItemObject.BP_BaseItemObject_C" self (make `IntPoint` (`KismetMathLibrary.FTrunc` _itemsize_x) (`KismetMathLibrary.FTrunc` _itemsize_y)) (`self.Icon`) (`self.Icon Rotate`) (`GameplayStatics.GetObjectClass` self) (`self.ItemInfo`) (`self.Amount`) (`self.Is Stack`) (`self.Weight`) (`self.Max Amount`) (`self.Is Usable?`) (`self.Item Action Type`) (`self.Equipment Class`)))
  (return _returnvalue))

(fn `UserConstructionScript`)