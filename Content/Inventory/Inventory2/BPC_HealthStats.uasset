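; Actor component that tracks current and maximum HP and the dead state for its owner in the inventory project.
; DoDamage subtracts from CurrentHP while alive, clamping the result at zero, and SetHP overwrites both values directly.
; Death is polled on Tick: when HP reaches zero, the Dead event fires once and sets IsDead.
; GetStatsForHUD supplies whole-number HP texts and a normalized fill value for a HUD progress bar.
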(event `Dead`
  (set `self.Is Dead?` true))

(event `self.ReceiveTick`
  (params (DeltaSeconds :type "Float (single-precision)"))
  (`self.CallDeadWhenHP=0`))

(fn `Do Damage`
  (params (Damage :type "Float (double-precision)"))
  (if (not (`self.Is Dead?`))
    (set `self.CurrentHP` (`KismetMathLibrary.SelectFloat` 0.0 (- (`self.CurrentHP`) Damage) (>= Damage (`self.CurrentHP`))))))

(fn `GetStatsForHUD`
  (returns (MaxHP :type Text) (CurrentHP :type Text) (HP_ProgressBar :type "Float (double-precision)"))
  (return (`KismetTextLibrary.Conv_Int64ToText` (`KismetMathLibrary.FTrunc64` (`self.MaxHP`))) (`KismetTextLibrary.Conv_Int64ToText` (`KismetMathLibrary.FTrunc64` (`self.CurrentHP`))) (`KismetMathLibrary.NormalizeToRange` (`self.CurrentHP`) 0.0 (`self.MaxHP`))))

(fn `SetHP`
  (params (SetMaxHP :type "Float (double-precision)") (SetCurrentHP :type "Float (double-precision)"))
  (set `self.MaxHP` SetMaxHP)
  (set `self.CurrentHP` SetCurrentHP))