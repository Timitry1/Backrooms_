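; BP_Useable is an inventory item actor for usable items that carry a health-to-add value.
; Its GetDefoultItemObject function constructs a BP_UsableItemObject owned by the actor, copying in its size, icons, info, stacking, weight and usability data along with its own class.
; The event graph is empty, and the construction script only calls the parent's.
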(fn `GetDefoultItemObject`
  (returns (ItemObject :type "/Game/Inventory/Inventory2/BP_BaseItemObject Object Reference"))
  (bind (_itemsize_x _itemsize_y) (`KismetMathLibrary.BreakVector2D` (`self.ItemSize`)))
  (bind _returnvalue (`|GenericCreateObject` "/Game/Inventory/Inventory2/Items/BP_UsableItemObject.BP_UsableItemObject_C" self (`self.Health to Add`) (make `IntPoint` (`KismetMathLibrary.FTrunc` _itemsize_x) (`KismetMathLibrary.FTrunc` _itemsize_y)) (`self.Icon`) (`self.Icon Rotate`) (`GameplayStatics.GetObjectClass` self) (`self.ItemInfo`) (`self.Amount`) (`self.Is Stack`) (`self.Weight`) (`self.Max Amount`) (`self.Is Usable?`) "(INVALID)" null))
  (return _returnvalue))

(fn `UserConstructionScript`
  (`parent.UserConstructionScript`))