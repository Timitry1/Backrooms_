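; BPC_Equipment is an equipment component Blueprint for the inventory, apparently meant to hold items in Hand, Head and Body slots.
; AddToEquip and RemoveEquip each take an item but are empty stubs.
; An unconnected switch in the AddToEquip graph would store the item in the matching slot only if it is empty.
; That switch never runs, and its selector is a fixed enum value rather than read from the item.
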(fn `AddToEquip`
  (params (`Item To Equip` :type "Object Object Reference")))

(fn `RemoveEquip`
  (params (ItemToRemove :type "Object Object Reference")))