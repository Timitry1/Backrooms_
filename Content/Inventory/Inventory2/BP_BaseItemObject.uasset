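; BP_BaseItemObject is the base item data object for the inventory, exposing icon, class, info, weight, stack amounts, usability and action type.
; It reports its 2D dimensions with X and Y swapped while rotated, and RotateIcon toggles that rotation flag.
; Most functions are simple getters, with setters for amount and weight.
; UseItem takes a player and is empty here.
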(fn `GetAmount`
  (returns (Amount :type Integer))
  (return (`self.Amount`)))

(fn `GetIsRotateIcon?`
  (returns (`IsRotate?` :type Boolean))
  (return (`self.IsRotate?`)))

(fn `GetIsStack?`
  (returns (IsStack :type Boolean))
  (return (`self.IsStack`)))

(fn `GetItemActionType`
  (returns (ItemActionType :type "/Game/Inventory/Inventory2/ItemType Enum"))
  (return (`self.ItemActionType`)))

(fn `GetItemClass`
  (returns (ItemClass :type "/Game/Inventory/Inventory2/BP_BaseInventoryItem Class Reference"))
  (return (`self.ItemClass`)))

(fn `GetItemDimension`
  (returns (Dimension :type "IntPoint Structure"))
  (bind (_dimension_x _dimension_y) (break `IntPoint` (`self.Dimension`)))
  (if (`self.IsRotate?`)
    (return (make `IntPoint` _dimension_y _dimension_x))
    (else
      (return (`self.Dimension`)))))

(fn `GetItemIcon`
  (returns (Icon :type "Texture2D Object Reference"))
  (return (`self.Icon`)))

(fn `GetItemInfo`
  (returns (ItemInfo :type "/Game/Inventory/Inventory2/ItemInfo Structure"))
  (return (`self.ItemInfo`)))

(fn `GetMaxAmount`
  (returns (MaxAmount :type Integer))
  (return (`self.MaxAmount`)))

(fn `GetUsable`
  (returns (`IsUsable?` :type Boolean))
  (return (`self.IsUsable?`)))

(fn `GetWeight?`
  (returns (Weight :type Integer))
  (return (`self.Weight`)))

(fn `RotateIcon`
  (set `self.IsRotate?` (not (`self.IsRotate?`)))
  (return))

(fn `SetAmount`
  (params (Amount :type Integer))
  (set `self.Amount` Amount)
  (return))

(fn `SetWeight`
  (params (Weight :type Integer))
  (set `self.Weight` Weight)
  (return))

(fn `UseItem`
  (params (Player :type "/Game/Main/Levels/Level0/Kentik/HUD/BP_GG Object Reference")))